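; BP_UIController creates the BP_UI widget and links it to hero and villain references.
; Tick waits for a valid HeroReference, creating the UI and binding the hero if the widget is missing, then binds a valid VillainReference behind a validity check with no visible input.
; SetUI lazily creates the widget, adds it to the viewport, and fills the hero or villain entity slot based on a boolean.
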(event `self.ReceiveTick`
  (params (DeltaSeconds :type "Float (single-precision)"))
  (`/Engine/EditorBlueprintResources/StandardMacros.IsValid` (`self.Hero Reference`)
    (:`Is Valid`
      (`/Engine/EditorBlueprintResources/StandardMacros.IsValid` (`self.UI`)
        (:`Is Valid`
          _)
        (:`Is Not Valid`
          (`self.Set UI` false)))
      (`/Engine/EditorBlueprintResources/StandardMacros.IsValid` (`self.Villain Reference`)
        (:`Is Valid`
          (`/Engine/EditorBlueprintResources/StandardMacros.IsValid` null
            (:`Is Not Valid`
              (`self.Set UI` true))))))))

(fn `Set UI`
  (params (isVillain :type Boolean))
  (`/Engine/EditorBlueprintResources/StandardMacros.IsValid` (`self.UI`)
    (:`Is Valid`
      _)
    (:`Is Not Valid`
      (bind _returnvalue (`|CreateWidget` "/Game/Test/BP/BP_UI.BP_UI_C"))
      (bind _output_get (set `self.UI` _returnvalue))
      (`UserWidget.AddToViewport` _output_get 0)))
  (if isVillain
    (set `/Game/Test/BP/BP_UI.Entity Reference_1` (`self.Villain Reference`) (`self.UI`))
    (else
      (set `/Game/Test/BP/BP_UI.Entity Reference` (`self.Hero Reference`) (`self.UI`)))))

(fn `UserConstructionScript`)