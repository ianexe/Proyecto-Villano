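; BP_Entity is a battle combatant that randomizes most stats on BeginPlay and automatically attacks its current enemy while battling.
; Tick checks for a win, then accumulates time to fire attacks at a Speed-based interval.
; Attacks use percentile rolls for critical, accuracy, evade and counterattack to decide damage, with debuffs lowering stats.
; A debug hook registers the instance with BP_UIController as villain or hero.
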(event `self.ReceiveBeginPlay`
  (`self.Set Initial Parameters`)
  ;[1 1 1] DEBUG - Set Entity Automatically to Controller
  (`self.ENTITY_DEBUG Set Instance to Controller`))

(event `self.ReceiveTick`
  (params (DeltaSeconds :type "Float (single-precision)"))
  (if (`self.is_battling`)
    (`self.Check Win`)
    (`self.Attack If Battling` DeltaSeconds)))

(fn `Attack If Battling`
  (params (`Delta Seconds` :type "Float (double-precision)"))
  (set `self.last_attack_delta` (+ (`self.last_attack_delta`) `Delta Seconds`))
  (if (>= (`self.last_attack_delta`) (`self.Time To Attack (Speed -> Time)`))
    (for _ (range 1 (+ (`KismetMathLibrary.FTrunc` (/ (`self.last_attack_delta`) (`self.Time To Attack (Speed -> Time)`))) 1))
      (`self.Do Attack` (`self.current_enemy`))
      (`KismetSystemLibrary.PrintString` "DO ATTACK" true true (struct :`R` 1.0 :`B` 0.433389 :`A` 1.0) 0.5))
    (set `self.last_attack_delta` 0.0)))

(fn `Check Damage`
  (params (`Enemy Critical` :type Integer) (`Enemy Accuracy` :type Integer))
  (returns (Attack_done :type Boolean) (Is_Critical :type Boolean) (Is_Counter :type Boolean))
  (locals (Critical_Return :type Boolean) (Attack_Return :type Boolean :default true) (Counter_Return :type Boolean))
  ;[1 1 1] Check Enemy Critical
  (bind _output_get (set `local.Critical_Return` (> `Enemy Critical` (`KismetMathLibrary.RandomIntegerInRange` 0 99))))
  (if (not _output_get)
    ;[1 1 1] Check Enemy Accuracy
    (bind _output_get_2 (set `local.Attack_Return` (> `Enemy Accuracy` (`KismetMathLibrary.RandomIntegerInRange` 0 99))))
    (if _output_get_2
      ;[1 1 1] Check Entity Evade
      (bind _output_get_3 (set `local.Attack_Return` (> (`KismetMathLibrary.RandomIntegerInRange` 0 99) (`self.Evade`))))
      (if _output_get_3
        ;[1 1 1] Check Entity Counterattack
        (set `local.Counter_Return` (> (`self.Counterattack`) (`KismetMathLibrary.RandomIntegerInRange` 0 99)))
        (else
          (`KismetSystemLibrary.PrintString` "Attack Evaded" true false)))
      (else
        (`KismetSystemLibrary.PrintString` "Attack Failed" true false (struct :`R` 1.0 :`G` 0.04934 :`B` 0.00954 :`A` 1.0)))))
  (return (`local.Attack_Return`) (`local.Critical_Return`) (`local.Counter_Return`)))

(fn `Check Win`
  (bind _current_enemy (`self.current_enemy`))
  (if (> (`self.Current HP`) 0)
    (if (`KismetSystemLibrary.IsValid` _current_enemy)
      (if (<= (`/Game/Test/BP/BP_Entity.Current HP` _current_enemy) 0)
        (set `self.is_battling` false)
        (set `self.is_win` true)
        (else
          (set `self.is_battling` true)
          (set `self.is_win` false))))
    (else
      (set `self.is_battling` false))))

(fn `Do Attack`
  (params (Enemy :type "/Game/Test/BP/BP_Entity Object Reference") (`Is Counter` :type Boolean))
  (if (not `Is Counter`)
    (bind (_attack_done _is_critical _is_counter) (`self.Check Damage` Enemy (`self.Critical`) (`self.Accuracy`)))
    (if _is_counter
      (`self.Receive Damage` false)
      (`KismetSystemLibrary.PrintString` "COUNTER!")
      (elif _attack_done
        (`self.Receive Damage` Enemy _is_critical)))))

(fn `ENTITY_DEBUG Set Instance to Controller`
  (bind _returnvalue (`GameplayStatics.GetActorOfClass` "/Game/Test/BP/BP_UIController.BP_UIController_C"))
  (`/Engine/EditorBlueprintResources/StandardMacros.IsValid` (`/Game/Test/BP/BP_UIController.Villain Reference` _returnvalue)
    (:`Is Valid`
      (`/Engine/EditorBlueprintResources/StandardMacros.IsValid` (`/Game/Test/BP/BP_UIController.Hero Reference` _returnvalue)
        (:`Is Not Valid`
          (set `/Game/Test/BP/BP_UIController.Hero Reference` self _returnvalue))))
    (:`Is Not Valid`
      (set `/Game/Test/BP/BP_UIController.Villain Reference` self _returnvalue))))

(fn `Receive Damage`
  (params (`Is Critical` :type Boolean))
  (locals (`Received Damage` :type Integer))
  (bind _returnvalue (- (`self.Current HP`) (`local.Received Damage`)))
  (if `Is Critical`
    (set `local.Received Damage` 2)
    (else
      (set `local.Received Damage` 1)))
  (if (< _returnvalue 0)
    (set `self.Current HP` 0)
    (else
      (set `self.Current HP` _returnvalue))))

(fn `Receive Debuff`
  (params (Value :type Integer) (`Parameter Type` :type "/Game/SideScrollerBP/Blueprints/ParameterType Enum" :default "NewEnumerator0"))
  (switch `/Game/SideScrollerBP/Blueprints/ParameterType` `Parameter Type`
    (:`NewEnumerator0`
      (set `self.Current HP` (- (`self.Current HP`) Value)))
    (:`NewEnumerator1`
      (set `self.Speed` (- (`self.Speed`) Value))
      (if (<= (`self.Speed`) 0)
        (set `self.Speed` 1)))
    (:`NewEnumerator2`
      (set `self.Accuracy` (- (`self.Accuracy`) Value)))
    (:`NewEnumerator3`
      (set `self.Evade` (- (`self.Evade`) Value)))
    (:`NewEnumerator4`
      (set `self.Counterattack` (- (`self.Counterattack`) Value)))))

(fn `Set Initial Parameters`
  (bind _output_get (set `self.Max HP` (`KismetMathLibrary.RandomIntegerInRange` 50 75)))
  (set `self.Current HP` _output_get)
  (set `self.Speed` (`KismetMathLibrary.RandomIntegerInRange` 5 10))
  (set `self.Evade` (`KismetMathLibrary.RandomIntegerInRange` 5 10))
  (set `self.Accuracy` (`KismetMathLibrary.RandomIntegerInRange` 75 100))
  (set `self.Counterattack` (`KismetMathLibrary.RandomIntegerInRange` 0 20))
  (set `self.Hazard Dodge` (`KismetMathLibrary.RandomIntegerInRange` 5 40)))

(fn `Set Parameters`
  (params (HP :type Integer) (Speed :type Integer) (Evade :type Integer) (Accuracy :type Integer) (Counterattack :type Integer) (Critical :type Integer) (`Hazard Dodge` :type Integer))
  (bind _output_get (set `self.Max HP` HP))
  (set `self.Current HP` _output_get)
  (set `self.Speed` Speed)
  (set `self.Evade` Evade)
  (set `self.Accuracy` Accuracy)
  (set `self.Counterattack` Counterattack)
  (set `self.Critical` Critical)
  (set `self.Hazard Dodge` `Hazard Dodge`))

(fn `Switch Battle Mode`
  (params (`New Enemy` :type "/Game/Test/BP/BP_Entity Object Reference") (`New Battle State` :type Boolean))
  (bind _output_get (set `self.is_battling` `New Battle State`))
  (if _output_get
    (set `self.current_enemy` `New Enemy`))
  (set `self.is_win` false))

(fn `UserConstructionScript`)